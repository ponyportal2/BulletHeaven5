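; BP_Guard is a pistol-armed enemy that spins while facing the player and fires when within range.
; It spawns hidden, reveals through a dissolve, and aims each tick by splitting look-at and roll across capsule and mesh gimbals.
; Timers drive periodic checks, while gravity-modulator events ease its custom time dilation.
; Death ragdolls and dissolves it, reporting player kills, melee hits and falls into space to the score counter.
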(event Custom|Dead
  (params (ByPlayer :type Boolean) (TimeDilAfterDeath :type Float%20%28single-precision%29) (Who :type Actor%20Object%20Reference) (ByHeadshot :type Boolean))
  ;[0 0.9062 1 0.5] Event Dead
  (if (not (Variables|Default|GetDeadBool))
    (if (== TimeDilAfterDeath 0.0)
      (Development|PrintString "GUARD TIME DILATION = 0, ERROR")
      (else
        (Variables|Default|SetDeadBool true)
        (if ByPlayer
          (Variables|Default|SetCustomTimeDilation TimeDilAfterDeath)
          (Audio|PlaySoundatLocation "/Game/AProject/Files/Audio/SC_brake_Cue.SC_brake_Cue" (Transformation|GetWorldLocation (Variables|Collision|GetCapsuleComponent)) "0, 0, 0" 1.0 1.0 0.0 0 0 0)
          (Class|BPIItoScores|PlayerKilledEnemy(Message) (Variables|Default|GetScoresCounterRef) false))
        (Class|SkeletalMeshComponent|SetAllBodiesSimulatePhysics (Variables|Default|GetCharacterMesh) true)
        (Collision|SetCollisionEnabled (Variables|Collision|GetCapsuleComponent) "NoCollision")
        (Variables|/Script/Engine.PrimitiveComponent|SetbGenerateOverlapEvents (Variables|Collision|GetCapsuleComponent) false)
        (bind _guardspistol (Variables|Default|GetGuardsPistol)
          (:then
            (Components|DestroyComponent _guardspistol)
            ;;[0 1 0.9766 0.5] Dissolve
            (CallFunction|Timer (EventDispatchers|CreateEvent :!event Custom|DestroyGuard) false 3.0)
            (bind _returnvalue (Rendering|Material|CreateDynamicMaterialInstance (Variables|Default|GetCharacterMesh) 0 "/Game/AProject/Files/CharacterModels/Biker/Materials/M_Biker_body_DIssolve_Inst.M_Biker_body_DIssolve_Inst" "None" :!class /Script/Engine.PrimitiveComponent))
            (Variables|Default|SetDynaMat _returnvalue)
            (Utilities|FlowControl|Delay 1.0)
            (bind _dissolve (Timeline|Dissolve PlayFromStart)
              (:Update
                (Rendering|Material|SetScalarParameterValue (Variables|Default|GetDynaMat) "DisolveAmount" _dissolve :!class /Script/Engine.MaterialInstanceDynamic))))
          (:else))))))

(event Custom|DestroyGuard
  ;[1 0 0.3516] DestroyGuard
  (Actor|DestroyActor))

(event Custom|UnHide
  ;[0.4531 1 0 0.3] Setup
  ;;[0.3594 1 0 0.3] Unhide
  (Utilities|2FramesDelay
    (:Completed
      (Rendering|SetActorHiddenInGame false)
      (bind _returnvalue (Rendering|Material|CreateDynamicMaterialInstance (Variables|Default|GetCharacterMesh) 0 "/Game/AProject/Files/Materials/Materialinst/MIC_GoldenDissolve_Inst.MIC_GoldenDissolve_Inst" "None" :!class /Script/Engine.PrimitiveComponent))
      (Variables|Default|SetDynaMat _returnvalue)
      (bind _dissolve (Timeline|Timeline_0 PlayFromStart)
        (:Update
          (Rendering|Material|SetScalarParameterValue (Variables|Default|GetDynaMat) "DisolveAmount" _dissolve :!class /Script/Engine.MaterialInstanceDynamic))
        (:Finished
          (Rendering|Material|SetMaterial (Variables|Default|GetCharacterMesh) 0 (Variables|Default|GetThatMat)))))))

(event Custom|DeleteIfLowerThan
  ;[1 0.6563 0] DeleteIfLowerThanEvent
  (if (and (<= (.z (Transformation|GetWorldLocation (Variables|Collision|GetCapsuleComponent))) -1.2e+03) (not (Variables|Default|GetDeadBool)))
    (Class|BPIItoScores|GuardLosttoSpace(Message) (Variables|Default|GetScoresCounterRef) false)
    (bind _guardspistol (Variables|Default|GetGuardsPistol)
      (:then
        (Components|DestroyComponent _guardspistol))
      (:else
        _))
    (Actor|DestroyActor)))

(event Custom|GravityModulatorEnd
  ;[1 0.8203 0] GravModulatorAndShootingTimer
  (if (not (Variables|Default|GetDeadBool))
    (bind _timedilationeasein (Timeline|TimeEaseIn Reverse)
      (:Update
        (Variables|Default|SetCustomTimeDilation _timedilationeasein)))))

(event Custom|GravityModulatorStart
  ;[1 0.8203 0] GravModulatorAndShootingTimer
  (if (not (Variables|Default|GetDeadBool))
    (Utilities|FlowControl|Sequence
      (:then_0
        (bind _timedilationeasein (Timeline|TimeEaseIn Play)
          (:Update
            (Variables|Default|SetCustomTimeDilation _timedilationeasein))))
      (:then_1
        (CallFunction|Timer (EventDispatchers|CreateEvent :!event Custom|CheckDistanceAndShootingOnGuard) true (CallFunction|LocalFloat 0.5))))))

(event Custom|CheckDistanceAndShootingOnGuard
  ;[0.1016 0 1 0.3] GuardShooting
  (if (< (CallFunction|GetDistance (Transformation|GetWorldLocation (Variables|Default|GetPlayerCapsule)) (Transformation|GetWorldLocation (Variables|Collision|GetCapsuleComponent)) false) (Variables|Default|GetPlayerNearDistance))
    (bind _guardspistol (Variables|Default|GetGuardsPistol)
      (:then
        (bind _asbp_pistol (Utilities|Casting|CastToBP_Pistol (Variables|/Script/Engine.ChildActorComponent|GetChildActor _guardspistol)))
        (Default|PistolShoot _asbp_pistol (Math|Rotator|FindLookatRotation (Transformation|GetWorldLocation (Variables|Default|GetGuardsPistol)) (Transformation|GetWorldLocation (Variables|Default|GetPlayerCapsule)))))
      (:else))))

(event EventBeginPlay
  ;[0.4531 1 0 0.3] Setup
  ;;[1 0.1172 0 0.5] BeginPlay
  (Rendering|SetActorHiddenInGame true)
  (bind _returnvalue (Rendering|Material|CreateDynamicMaterialInstance (Variables|Default|GetCharacterMesh) 0 "/Game/AProject/Files/CharacterModels/Biker/Materials/MIC_Biker_body_Inst.MIC_Biker_body_Inst" "None" :!class /Script/Engine.PrimitiveComponent))
  (bind _output_get (Variables|Default|SetThatMat _returnvalue))
  (Rendering|Material|SetVectorParameterValue _output_get "RandColor" (Variables|Default|GetRandColor) :!class /Script/Engine.MaterialInstanceDynamic)
  (Variables|Default|SetRandLeftRightPlusOneRot (Math|Float|Clamp(Float) (* (Math|Random|RandomFloatinRange (Variables|Default|GetMinRandomRot) (Variables|Default|GetMaxRandomRot)) (Variables|Default|GetRandRotMultiplier)) -1.5 1.5))
  (Variables|Default|SetRandRot (Math|Conversions|ToFloat(Integer) (Math|Random|RandomIntegerinRange -359 359)))
  ;;[0 1 0.9766 0.3] Getters
  (bind _playercapsule (Utilities|GetPlayerCapsule))
  (Variables|Default|SetPlayerCapsule _playercapsule)
  (bind _asscores_counter (Utilities|GetScoresCoutner))
  (Variables|Default|SetScoresCounterRef _asscores_counter)
  (Variables|Default|SetPlayerCapLocation (Transformation|GetWorldLocation (Variables|Default|GetPlayerCapsule)))
  (Actor|Tick|SetActorTickEnabled true)
  (CallFunction|Timer (EventDispatchers|CreateEvent :!event Custom|DeleteIfLowerThan) true 0.5)
  (CallFunction|Timer (EventDispatchers|CreateEvent :!event Custom|UnHide) false 0.3)
  (CallFunction|Timer (EventDispatchers|CreateEvent :!event Custom|CheckDistanceAndShootingOnGuard) true 0.1))

(event EventTick
  (params (DeltaSeconds :type Float%20%28single-precision%29))
  ;[0 0.2031 1 0.5] Tick
  (bind _roll (CallFunction|PlusRotation))
  (Variables|Default|SetTempRoll _roll)
  (bind _returnvalue (CallFunction|LookatPlayer 0.0 false))
  (CallFunction|SetBothGimbalsRotation (Variables|Collision|GetCapsuleComponent) (Variables|Character|GetMesh) (.yaw _returnvalue) (.pitch _returnvalue) (Variables|Default|GetTempRoll)))

(fn ConstructionScript
  ;[0.007812 0 1 0.5] BeginPlay
  ;[1 0 0.6328 0.3] Needed Variables
  (Variables|Default|SetHealth (Variables|Default|GetHealth)))

(fn PlusRotation
  (bind _output_get (Variables|Default|SetRandRot (|(a+(b*c)) (Variables|Default|GetRandRot) (Variables|Default|GetRandLeftRightPlusOneRot) (Math|Random|RandomFloat))))
  (return _output_get))

(fn LookatPlayer
  (params (X%20%28Roll%29%20If%20Rendered :type Float%20%28single-precision%29) (rendered :type Boolean))
  (bind _playercapsule (Variables|Default|GetPlayerCapsule))
  (bind _capsulecomponent (Variables|Collision|GetCapsuleComponent))
  (bind _returnvalue (Transformation|GetWorldLocation _capsulecomponent))
  (bind _returnvalue_2 (Transformation|GetWorldLocation _playercapsule))
  (bind _returnvalue_3 (* (.x _returnvalue_2) -1.0))
  (bind _returnvalue_4 (* (.x _returnvalue) -1.0))
  (bind _returnvalue_5 (Math|Rotator|FindLookatRotation (Math|Vector|MakeVector (.z _returnvalue) (.y _returnvalue) _returnvalue_4) (Math|Vector|MakeVector (.z _returnvalue_2) (.y _returnvalue_2) _returnvalue_3)))
  (return (Math|Rotator|MakeRotator (.roll _returnvalue_5) (* (+ (.pitch _returnvalue_5) -9e+01) -1.0) (.yaw _returnvalue_5))))

(fn Loog
  (params (From :type Vector) (To :type Vector))
  (bind _returnvalue (Math|Vector|Normalize To))
  (bind _returnvalue_2 (Math|Vector|Normalize From))
  (bind _returnvalue_3 (Math|Vector|CrossProduct _returnvalue_2 _returnvalue))
  (bind _returnvalue_4 (Math|Vector|DotProduct _returnvalue_2 _returnvalue))
  (bind _returnvalue_5 (Class|KismetMathLibrary|DegAcos _returnvalue_4))
  (bind _returnvalue_6 (Math|Vector|RotatorfromAxisandAngle _returnvalue_3 _returnvalue_5))
  (return (Math|Rotator|MakeRotator (.roll _returnvalue_6) (+ (.pitch _returnvalue_6) -9e+01) (.yaw _returnvalue_6))))

(fn LookatPlayer2
  (params (X%20%28Roll%29%20If%20Rendered :type Float%20%28single-precision%29) (rendered :type Boolean))
  (bind _playercapsule (Variables|Default|GetPlayerCapsule))
  (bind _capsulecomponent (Variables|Collision|GetCapsuleComponent))
  (bind _returnvalue (Transformation|GetWorldLocation _capsulecomponent))
  (bind _returnvalue_2 (Transformation|GetWorldLocation _playercapsule))
  (bind _returnvalue_3 (* (.x _returnvalue_2) -1.0))
  (bind _returnvalue_4 (* (.y _returnvalue) -1.0))
  (bind _returnvalue_5 (Math|Rotator|FindLookatRotation (Math|Vector|MakeVector _returnvalue_4 (.x _returnvalue) (.z _returnvalue)) (Math|Vector|MakeVector (.y _returnvalue_2) _returnvalue_3 (.z _returnvalue_2))))
  (return (Math|Rotator|MakeRotator (.roll _returnvalue_5) (.pitch _returnvalue_5) (- (.yaw _returnvalue_5) -9e+01)) "0, 0, 0"))

(fn SetBothGimbalsRotation
  (params (CapsGimb :type Scene%20Component%20Object%20Reference) (MeshGimb :type Scene%20Component%20Object%20Reference) (NewRotation_Yaw :type Float%20%28single-precision%29) (NewRotation_Pitch :type Float%20%28single-precision%29) (Roll :type Float%20%28single-precision%29))
  (Transformation|SetWorldRotation CapsGimb (Math|Rotator|MakeRotator 0.0 NewRotation_Pitch 0.0) false false)
  (Transformation|SetRelativeRotation MeshGimb (Math|Rotator|MakeRotator Roll 0.0 NewRotation_Yaw) false false)
  (return))

(fn OverlappedwithPlayer
  (params (Who :type Actor%20Object%20Reference))
  (Class|BPIItoScores|HitbyMelee(Message) (Variables|Default|GetScoresCounterRef) false)
  (CallFunction|Dead true 1.0 0 false)
  (Physics|AddImpulse (Variables|Default|GetCharacterMesh) "0, 0,200000.000000" "None" true)
  (return true false))