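; Spawner Blueprint that places random satellites in space, built on a parent spawner class.
; BeginPlay converts the SatelitesTypes collection into an array of classes.
; Spawn picks a random class from that array and spawns it at a point from the inherited random-in-box function, with random rotation up to 90 degrees per axis, adjusting for collisions but always spawning.
; Some leftover random-direction math is unconnected.
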(event EventBeginPlay
  (|CallParentFunction)
  (bind _result (Utilities|Set|ToArray (Variables|Default|GetSatelitesTypes)))
  (Variables|Default|SetSatelliteTypesArray _result))

(event EventSpawn
  (bind _returnvalue (Math|Random|RandomFloat))
  (bind _returnvalue_2 (* _returnvalue 9e+01))
  (Game|SpawnActorfromClass (Utilities|Array|Get(acopy) (Variables|Default|GetSatelliteTypesArray) (Math|Random|RandomIntegerinRange 0 (Utilities|Array|LastIndex (Variables|Default|GetSatelliteTypesArray)))) (Math|Transform|MakeTransform (.location (Math|Conversions|ToTransform(Vector) (CallFunction|RandominBoxNoOverride))) (Math|Rotator|MakeRotator _returnvalue_2 _returnvalue_2 _returnvalue_2) "1,1,1") "AdjustIfPossibleButAlwaysSpawn" 0 0))

(fn ConstructionScript
  (|CallParentFunction))

(fn RandominBoxNoOverride
  (return (|CallParentFunction)))