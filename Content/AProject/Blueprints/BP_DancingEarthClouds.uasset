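; Earth clouds actor that reacts to audio frequency values by pulsing brightness and shifting color.
; The construction script creates a dynamic cloud material instance, and BeginPlay binds to a frequency analyzer's dispatcher.
; Each received value maps to initial brightness, scaled by a PC multiplier, and picks a random hue that keeps LinearColor's saturation and value.
; The Windows check that would raise that multiplier is unconnected and never runs.
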(event Custom|FreqReceived
  (params (FreqValue :type Float%20%28single-precision%29) (WorldTimeDilation :type Float%20%28single-precision%29))
  (bind _pcmultiplier (Variables|Default|GetPCMultiplier))
  (bind _linearcolor (Variables|Default|GetLinearColor))
  (bind _returnvalue (Class|KismetMathLibrary|RGBLineartoHSV _linearcolor))
  (bind (_r _g _b _a) (Utilities|Struct|BreakLinearColor _returnvalue))
  ;[0 0.9766 1 0.3] AssignOnFreqDispatch
  ;;[0 1 0.9766 0.3] Getter
  (bind _output_get (Variables|Default|SetFreqValue FreqValue))
  ;[0.3125 0 1 0.3] LightAndShitDOP
  (Rendering|Material|SetScalarParameterValue (Variables|Default|GetDynaMat) "InitialBrightness" (Math|Float|MapRangeClamped _output_get 0.0 (* 7.5 _pcmultiplier) -1.0 (* 4.0 _pcmultiplier)) :!class /Script/Engine.MaterialInstanceDynamic)
  ;[1 0 0.4922 0.3] RandomHue
  (Rendering|Material|SetVectorParameterValue (Variables|Default|GetDynaMat) "Param" (Class|KismetMathLibrary|HSVtoRGB (Math|Conversions|ToFloat(Integer) (Math|Random|RandomIntegerinRange 24 290)) _g _b _a) :!class /Script/Engine.MaterialInstanceDynamic))

(event EventBeginPlay
  ;[0 0.9766 1 0.3] AssignOnFreqDispatch
  ;;[0 0.2969 1 0.3] BeginPlay
  (bind _freq_analyzerref (Utilities|GetFreqAnalyzer))
  (EventDispatchers|BindEventtoCallFreqDispatch _freq_analyzerref (delegate Custom|FreqReceived)))

(event Collision|EventActorBeginOverlap
  (params (OtherActor :type Actor%20Object%20Reference)))

(event EventTick
  (params (DeltaSeconds :type Float%20%28single-precision%29)))

(fn ConstructionScript
  (bind _returnvalue (Rendering|Material|CreateDynamicMaterialInstance (Variables|Debug|GetStaticMeshComponent) 0 "/Game/AProject/Files/Materials/Materialinst/MIC_EarthClouds_Inst.MIC_EarthClouds_Inst" "None" :!class /Script/Engine.PrimitiveComponent))
  (Variables|Default|SetDynaMat _returnvalue))