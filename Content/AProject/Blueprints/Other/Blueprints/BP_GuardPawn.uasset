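; BP_GuardPawn is a guard pawn that turns its Sphere to track the player's capsule.
; Each tick it computes a look-at rotation from Sphere to PlayerCapsule using remapped world axes, swapping X and Z and negating X.
; ChangeBothRot applies it as the Sphere's relative rotation with a pitch offset and prints the angles for debugging.
; The node that sets PlayerCapsule is disconnected, and BeginPlay is empty.
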(event EventTick
  (params (DeltaSeconds :type Float%20%28single-precision%29))
  (bind _playercapsule (Variables|Default|GetPlayerCapsule))
  (bind _sphere (Variables|Default|GetSphere))
  (bind _returnvalue (Transformation|GetWorldLocation _sphere))
  (bind _returnvalue_2 (Transformation|GetWorldLocation _playercapsule))
  (bind _returnvalue_3 (* (.x _returnvalue_2) -1.0))
  (bind _returnvalue_4 (* (.x _returnvalue) -1.0))
  (bind _returnvalue_5 (Math|Rotator|FindLookatRotation (Math|Vector|MakeVector (.z _returnvalue) (.y _returnvalue) _returnvalue_4) (Math|Vector|MakeVector (.z _returnvalue_2) (.y _returnvalue_2) _returnvalue_3)))
  (CallFunction|ChangeBothRot (.roll _returnvalue_5) (.pitch _returnvalue_5) (.yaw _returnvalue_5)))

(event EventBeginPlay)

(fn ConstructionScript)

(fn ChangeBothRot
  (params (NewRotation_Roll :type Float%20%28single-precision%29) (NewRotation_Pitch :type Float%20%28single-precision%29) (NewRotation_Yaw :type Float%20%28single-precision%29))
  (Transformation|SetRelativeRotation (Variables|Default|GetSphere) (Math|Rotator|MakeRotator NewRotation_Roll (+ NewRotation_Pitch -9e+01) NewRotation_Yaw) false false)
  (Development|PrintString (Utilities|String|Append (Utilities|String|ToString(Integer) (Math|Float|Truncate NewRotation_Roll)) " ; " (Utilities|String|ToString(Integer) (Math|Float|Truncate NewRotation_Pitch)) " ; " (Utilities|String|ToString(Integer) (Math|Float|Truncate NewRotation_Yaw))))
  (return))