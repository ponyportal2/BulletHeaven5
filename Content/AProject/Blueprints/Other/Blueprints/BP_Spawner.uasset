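; BP_Spawner is an actor that continuously populates its box volume with guards and abstract "Sat" actors.
; From BeginPlay, a looping timer drives a FlipFlop that alternates between spawning BP_Guard and BP_SatAbstract at random points in the box.
; BP_SatAbstract also gets a random rotation and scale.
; The game-menu start binding is disconnected and its handler is empty, so spawning ignores game start.
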(event Custom|CreateGuard
  (bind _box (Variables|Default|GetBox))
  (bind _box_2 (Variables|Default|GetBox))
  (bind _returnvalue (Transformation|GetWorldLocation _box))
  (bind _returnvalue_2 (Components|Box|GetScaledBoxExtent _box_2))
  (bind _returnvalue_3 (Math|Random|RandomPointinBoundingBox _returnvalue _returnvalue_2))
  (bind _returnvalue_4 (Math|Conversions|ToTransform(Vector) _returnvalue_3))
  ;[0 0.4609 1 0.3] CreateGuard
  (Utilities|FlowControl|FlipFlop
    (:A
      (Game|SpawnActorfromClass "/Game/AProject/Blueprints/Main/BP_Guard.BP_Guard_C" (Math|Conversions|ToTransform(Vector) _returnvalue_3) "AdjustIfPossibleButAlwaysSpawn" 0 0))
    (:B
      (Game|SpawnActorfromClass "/Game/AProject/Blueprints/BP_SatAbstract.BP_SatAbstract_C" (Math|Transform|MakeTransform (.location _returnvalue_4) (Math|Conversions|RotationFromXVector (* (Math|Random|RandomUnitVector) 3.6e+02)) (* (.scale _returnvalue_4) (Math|Random|RandomFloatinRange 1.0 3.0))) "AdjustIfPossibleButAlwaysSpawn" 0 0))))

(event Custom|GameStartedEvent
  (params (TrackNumber :type Integer))
  ;[0 0 0] Setup with GetterDOP
)

(event EventBeginPlay
  ;[0.875 1 0 0.3] BeginPlay
  (CallFunction|Timer (delegate Custom|CreateGuard) true 0.75))

(fn ConstructionScript)