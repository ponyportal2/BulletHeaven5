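; BP_Spawner_Skyscrappers is a child spawner Blueprint that spawns BP_Guard actors.
; Its Spawn event places each guard at a random box point, adjusting for collisions where possible but always spawning.
; It overrides RandomInBoxNoOverride to double the vector returned by the parent's version.
; BeginPlay and the construction script only call the parent, and nothing in this graph triggers Spawn.
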(event EventBeginPlay
  (|CallParentFunction))

(event EventSpawn
  (Game|SpawnActorfromClass "/Game/AProject/Blueprints/BP_Guard.BP_Guard_C" (Math|Conversions|ToTransform(Vector) (CallFunction|RandominBoxNoOverride)) "AdjustIfPossibleButAlwaysSpawn" 0 0))

(fn ConstructionScript
  (|CallParentFunction))

(fn RandominBoxNoOverride
  (return (* (|CallParentFunction) 2.0)))