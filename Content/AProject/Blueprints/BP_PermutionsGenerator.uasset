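; BP_PermutionsGenerator is a Blueprint named for generating permutations, though its graph only concatenates and prints array elements.
; On BeginPlay, a fixed loop of roughly ten thousand passes walks InpudArray in order, appending each element as text to TempFinalStringArray.
; The growing string is printed several times after every append and is never cleared or reordered, so no permutations are produced.
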(event EventBeginPlay
  (for _index (range 0 10000)
    (for _array_element (Variables|Default|GetInpudArray)
      (bind _output_get (Variables|Default|SetTempFinalStringArray (Utilities|String|Append (Variables|Default|GetTempFinalStringArray) (Utilities|String|ToString(Integer) _array_element))))
      (Development|PrintString _output_get)
      (Development|PrintString _output_get)
      (Development|PrintString _output_get)
      (Development|PrintString _output_get))))

(fn ConstructionScript)