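; ProjectileBase is an actor Blueprint for a projectile that destroys itself one second after BeginPlay.
; OverlappedWithPlayer sends a player-hit message to the score counter and returns false for Dead and SateliteHit.
; Nothing here calls that function, and the Box overlap event is empty.
; An unwired Debug macro would, after a short delay, call GotIt on the first GearVRPawn found.
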(event OnComponentBeginOverlap(Box)
  (params (OverlappedComponent :type Primitive%20Component%20Object%20Reference) (OtherActor :type Actor%20Object%20Reference) (OtherComp :type Primitive%20Component%20Object%20Reference) (OtherBodyIndex :type Integer) (bFromSweep :type Boolean) (SweepResult :type Hit%20Result%20Structure%20%28by%20ref%29)))

(event EventBeginPlay
  ;[0 0.9297 1 0.3] BeginPlay
  ;[0 1 0.3906 0.3] DestroyProjectile
  (Utilities|FlowControl|Delay 1.0)
  (Actor|DestroyActor))

(fn ConstructionScript
  ;[1 0.7734 0 0.3] Needed Variables
  (Variables|Default|SetPlayerRef (Variables|Default|GetPlayerRef)))

(fn OverlappedwithPlayer
  (params (Who :type Actor%20Object%20Reference))
  (bind _asscores_counter (Utilities|GetScoresCoutner))
  (Class|ItoScores|PlayerGotHit(Message) _asscores_counter false)
  (return false false))