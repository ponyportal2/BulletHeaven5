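; Music analyzer actor that plays the track chosen at game start and turns its frequency magnitudes into light values and global time dilation.
; Tick samples submix frequencies and dispatches a scaled light magnitude with a dilation value mapped inversely from the first band.
; A looping timer, pausable by events, smooths that dilation by lerp and applies it globally.
; When the track finishes, it prints the VR pawn's hit percentage.
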(event Custom|TimeDilationSmooth
  ;[0 0.2031 1 0.5] Dilation
  (bind _output_get (Variables|Default|SetTimeDil (Math|Float|Lerp (* (Variables|Default|GetTimeDil) 1.0) (Math|Float|MapRangeClamped (Utilities|Array|Get(acopy) (stale EventTick _output_get)) 0.0 (Variables|Default|GetTimeDilationFromMusicMultiplier) 1.0 0.1) 0.5)))
  (Utilities|Time|SetGlobalTimeDilation _output_get))

(event Custom|ResumeDilation
  ;[0 0.2031 1 0.5] Dilation
  ;;[0 1 0.4375 0.5] PauseResumeDilationTimer
  (Utilities|Time|UnpauseTimerbyHandle (stale EventBeginPlay _returnvalue)))

(event Custom|GameStartedEvent
  (params (TrackNumber :type Integer))
  ;[0 0.8359 1 0.5] Setup
  ;;[0 1 0.5781 0.5] GameStartedEvent
  (Actor|Tick|SetActorTickEnabled true)
  (bind _returnvalue (Audio|SpawnSound2D (Utilities|Array|Get(acopy) (Variables|Default|GetMusicTracksArray) TrackNumber) 1.0 1.0 0.0 0))
  (EventDispatchers|AssignOnAudioFinished _returnvalue (delegate Custom|OnAudioFinished_Event_0)))

(event Custom|PauseDilation
  ;[0 0.2031 1 0.5] Dilation
  ;;[0 1 0.4375 0.5] PauseResumeDilationTimer
  (Utilities|Time|PauseTimerbyHandle (stale EventBeginPlay _returnvalue)))

(event Custom|OnAudioFinished_Event_0
  ;[0 0.8359 1 0.5] Setup
  (bind _outactors (Actor|GetAllActorsOfClass "/Game/AProject/Blueprints/BP_GearVRPawn.BP_GearVRPawn_C"))
  (bind _asbp_gear_vrpawn (Utilities|Casting|CastToBP_GearVRPawn (Utilities|Array|Get(acopy) _outactors)))
  (Development|PrintString (Utilities|String|ToString(Float) (|((a/(a+b))*100) (Variables|/Game/AProject/Blueprints/BP_GearVRPawn.BP_GearVRPawn_C|GetIHitTheGuardCounter _asbp_gear_vrpawn) (Variables|/Game/AProject/Blueprints/BP_GearVRPawn.BP_GearVRPawn_C|GetIMissedCounter _asbp_gear_vrpawn)))))

(event EventBeginPlay
  ;[0.07812 0 1 0.5] BeginPlay
  (Variables|Default|SetLightsMultiplier (* (Variables|Default|GetLightsMultiplier) (Variables|Default|GetLightsPCMultiplier)))
  ;[0 0.8359 1 0.5] Setup
  (bind _result (Utilities|Set|ToArray (Variables|Default|GetMusicTracksSet)))
  ;;[0.4062 0 1 0.5] Getter
  (Variables|Default|SetMusicTracksArray _result)
  (bind _asgame_menu (Utilities|GetGameMenu))
  (EventDispatchers|AssignGameStarted _asgame_menu (delegate Custom|GameStartedEvent))
  ;;[0 1 0.1094 0.5] Prefill Magnitudes Array With Zeroes
  (for (_ _array_index) (Variables|Default|GetFrequenciesToAnalyze)
    (Utilities|Array|SetArrayElem (Variables|Default|GetLatestMagnitudes) _array_index 0.0 true)
    ;[0 0.2031 1 0.5] Dilation
    ;;[1 0 0.375 0.5] Start Analyzing Submix Output
    (Class|AudioMixerBlueprintLibrary|StartAnalyzingOutput (Variables|Default|GetSubmixToAnalyze))
    (bind _returnvalue (Utilities|Time|SetTimerbyEvent (delegate Custom|TimeDilationSmooth) 0.07 true))))

(event Collision|EventActorBeginOverlap
  (params (OtherActor :type Actor%20Object%20Reference))
  ;[1 0.4453 0 0.5] Get Latest Magnitudes
)

(event EventTick
  (params (DeltaSeconds :type Float%20%28single-precision%29))
  ;[1 0.4453 0 0.5] Get Latest Magnitudes
  ;;[1 0 0.6797 0.5] Tick
  (bind _magnitudes (Class|AudioMixerBlueprintLibrary|GetMagnitudeforFrequencies (Variables|Default|GetFrequenciesToAnalyze) (Variables|Default|GetSubmixToAnalyze)))
  (bind _output_get (Variables|Default|SetLatestMagnitudes _magnitudes))
  ;;[0 0.0625 1 0.5] Dispatcher
  (Default|CallCallFreqDispatch (* (Utilities|Array|Get(acopy) _output_get 7) (Variables|Default|GetLightsMultiplier)) (Math|Float|MapRangeClamped (Utilities|Array|Get(acopy) _output_get) 0.0 (Variables|Default|GetTimeDilationFromMusicMultiplier) 1.0 0.1)))

(fn ConstructionScript)