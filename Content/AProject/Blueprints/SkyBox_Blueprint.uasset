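; Skybox Blueprint that makes the sky gradient pulse with values from a frequency analyzer, presumably audio-driven.
; The construction script creates a dynamic instance of the gradient material on the static mesh.
; BeginPlay binds to the analyzer's frequency dispatch, whose handler maps each value through a clamped range, scaled by PCMultiplier, into the material's Power parameter.
; Windows-specific multiplier and random-hue logic exist but are disconnected.
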(event Custom|FreqReceived
  (params (FreqValue :type Float%20%28single-precision%29) (WorldTimeDilation :type Float%20%28single-precision%29))
  ;[0.2656 1 0 0.3] Getter
  (bind _output_get (Variables|Default|SetFreqValue FreqValue))
  (Rendering|Material|SetScalarParameterValue (Variables|Default|GetDynaMat) "Power" (Math|Float|MapRangeClamped _output_get 0.0 (* 15.0 1.0) -12.0 (* 4.0 (Variables|Default|GetPCMultiplier))) :!class /Script/Engine.MaterialInstanceDynamic))

(event EventBeginPlay
  (Variables|Default|SetPCMultiplier 6.0)
  (bind _freq_analyzerref (Utilities|GetFreqAnalyzer))
  (EventDispatchers|BindEventtoCallFreqDispatch _freq_analyzerref (delegate Custom|FreqReceived)))

(event EventTick
  (params (DeltaSeconds :type Float%20%28single-precision%29))
  ;[0.7813 0 1 0.3] Tick
)

(fn ConstructionScript
  (bind _returnvalue (Rendering|Material|CreateDynamicMaterialInstance (Variables|Debug|GetStaticMeshComponent) 0 "/Game/AProject/Assets/Materialinst/SkyBoxGradient_Inst.SkyBoxGradient_Inst" "None" :!class /Script/Engine.PrimitiveComponent))
  (Variables|Default|SetDynaMat _returnvalue))