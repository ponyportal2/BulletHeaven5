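; Spawner Blueprint that randomly places either a BP_Guard or a BP_SatAbstract actor at a random point in a box.
; The Spawn event picks one class with equal odds and gets its location from RandomInBoxNoOverride.
; Guards receive only a random-vector-derived roll, while SatAbstracts derive roll, pitch and yaw that way.
; Spawns adjust to avoid collisions or are skipped, and BeginPlay and construction defer to the parent.
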(event EventBeginPlay
  (|CallParentFunction))

(event EventSpawn
  (bind _returnvalue (CallFunction|RandominBoxNoOverride))
  (bind _returnvalue_2 (Math|Random|RandomUnitVector))
  (bind _returnvalue_3 (* _returnvalue_2 3.6e+02))
  (bind _returnvalue_4 (Math|Conversions|RotationFromXVector _returnvalue_3))
  (switch int (Math|Random|RandomInteger 2)
    (:0
      (Game|SpawnActorfromClass "/Game/AProject/Blueprints/Main/BP_Guard.BP_Guard_C" (Math|Transform|MakeTransform (.location (Math|Conversions|ToTransform(Vector) _returnvalue)) (Math|Rotator|MakeRotator (.roll _returnvalue_4) 0.0 0.0) "1,1,1") "AdjustIfPossibleButDontSpawnIfColliding" 0 0))
    (:1
      (Game|SpawnActorfromClass "/Game/AProject/Blueprints/BP_SatAbstract.BP_SatAbstract_C" (Math|Transform|MakeTransform (.location (Math|Conversions|ToTransform(Vector) _returnvalue)) (Math|Rotator|MakeRotator (.roll _returnvalue_4) (.pitch _returnvalue_4) (.yaw _returnvalue_4)) "1,1,1") "AdjustIfPossibleButDontSpawnIfColliding" 0 0))))

(fn ConstructionScript
  (|CallParentFunction))