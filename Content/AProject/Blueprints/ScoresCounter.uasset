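; ScoresCounter is a stat-tracking Blueprint that tallies combat events for scoring.
; Separate functions increment counters for guards lost to space, enemies hit by melee, player bullet hits taken and enemy kills, with headshot kills also counted separately.
; Each function always returns false, and nothing in this file reads the totals or turns them into a score.
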(fn ConstructionScript
  ;[0 0.5312 1 0.3] Needed Variables
  (Variables|Default|SetPlayerGotHitByBulletCounter (Variables|Default|GetPlayerGotHitByBulletCounter)))

(fn GuardLosttoSpace
  (params (in :type Boolean))
  (Math|Integer|IncrementInt (Variables|Default|GetEnemyLostToSpaceCount)
    (:%20%20
      (return false))))

(fn HitbyMelee
  (params (In :type Boolean))
  (Math|Integer|IncrementInt (Variables|Default|GetEnemyHitByMeleeCount)
    (:%20%20
      (return false))))

(fn PlayerGotHit
  (params (Dummy :type Boolean))
  (Math|Integer|IncrementInt (Variables|Default|GetPlayerGotHitByBulletCounter)
    (:%20%20
      (return false))))

(fn PlayerKilledEnemy
  (params (Head%20shot :type Boolean))
  (Math|Integer|IncrementInt (Variables|Default|GetKilledEnemyCount)
    (:%20%20
      (if Head%20shot
        (Math|Integer|IncrementInt (Variables|Default|GetKilledByHeadShotCount)
          (:%20%20
            _)))
      (return false))))