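; A Blueprint utility library of small reusable helpers for flow control, timers, component lookup and math.
; The gate helpers continue only when a condition holds or an actor has a valid component of a given class, which is also returned.
; Other helpers wrap timer-by-event setup, return a float array's min and max together, and output incremented int or float copies without modifying the input.
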(fn IfGate
  (params (Condition :type Boolean))
  (if Condition
    (return)))

(fn Timer
  (params (Event :type Delegate) (bLooping :type Boolean) (Time :type Float%20%28single-precision%29))
  (bind _returnvalue (Utilities|Time|SetTimerbyEvent Event Time bLooping))
  (return _returnvalue))

(fn ActorHasComponentGate
  (params (Actor :type Actor%20Object%20Reference) (ComponentClass :type Actor%20Component%20Class%20Reference))
  (bind _returnvalue (Actor|GetComponentbyClass Actor ComponentClass))
  (if (Utilities|IsValid _returnvalue)
    (return _returnvalue)))

(fn ArrayMinMaxFloat
  (params (FloatArray :type Array%20of%20Floats%20%28single-precision%29))
  (return (.MinValue (Math|Float|MinOfFloatArray FloatArray)) (.MaxValue (Math|Float|MaxOfFloatArray FloatArray))))

(fn IncrementIntCopy
  (params (In :type Integer))
  (return (+ In 1)))

(fn IncrementFloatCopy
  (params (In :type Float%20%28single-precision%29))
  (return (+ In 1.0)))