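; Blueprint utility library of general-purpose shorthand helpers that wrap common engine nodes.
; Gate helpers branch on conditions, object validity or component presence, alongside a timer-by-event wrapper.
; Lookups pick the first, indexed or random actor of a class without empty-array checks, or filter components by tag.
; Line-trace wrappers start from a target's world location, with small location, float and string-append helpers rounding out the set.
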(fn IfGate
  (params (Condition :type Boolean))
  (if Condition
    (return)))

(fn Timer
  (params (Event :type Delegate) (bLooping :type Boolean) (Time :type Float%20%28single-precision%29))
  (bind _returnvalue (Utilities|Time|SetTimerbyEvent Event Time bLooping))
  (return _returnvalue))

(fn ActorHasComponentGate
  (params (Actor :type Actor%20Object%20Reference) (ComponentClass :type Actor%20Component%20Class%20Reference))
  (bind _returnvalue (Actor|GetComponentbyClass Actor ComponentClass))
  (if (Utilities|IsValid _returnvalue)
    (return _returnvalue)))

(fn GetFirstActorOfClass
  (params (ActorClass :type Actor%20Class%20Reference))
  (bind _outactors (Actor|GetAllActorsOfClass 0 ActorClass))
  (return (Utilities|Array|Get(acopy) _outactors)))

(fn GetConcreteActorOfClass
  (params (ActorClass :type Actor%20Class%20Reference) (ActorNum :type Integer))
  (bind _outactors (Actor|GetAllActorsOfClass 0 ActorClass))
  (return (Utilities|Array|Get(acopy) _outactors ActorNum)))

(fn GetRandomActorOfClass
  (params (ActorClass :type Actor%20Class%20Reference))
  (bind _outactors (Actor|GetAllActorsOfClass 0 ActorClass))
  (return (Utilities|Array|Get(acopy) _outactors (Math|Random|RandomIntegerinRange 0 (Utilities|Array|LastIndex _outactors)))))

(fn ConnectorFloat
  (params (In :type Float%20%28single-precision%29))
  (return 0.0))

(fn FindTaginComponents
  (params (Comps :type Array%20of%20Actor%20Component%20Object%20References) (Tag :type Name%20%28by%20ref%29))
  (for _array_element Comps
    (if (Utilities|Array|ContainsItem (Variables|/Script/Engine.ActorComponent|GetComponentTags _array_element) Tag)
      (Utilities|Array|Add (LocalVariables|GetWithTag) _array_element)))
  (return (LocalVariables|GetWithTag)))

(fn TracebyChfromTwoActors
  (params (FromActor :type Scene%20Component%20Object%20Reference) (ToActor :type Scene%20Component%20Object%20Reference) (TraceChannel :type ETraceTypeQuery%20Enum :default "TraceTypeQuery1") (bTraceComplex :type Boolean) (ActorsToIgnore :type Array%20of%20Actor%20Object%20References) (DrawDebugType :type EDrawDebugTrace%20Enum :default "None") (IgnoreSelf :type Boolean) (TraceColor :type Linear%20Color%20Structure) (TraceHitColor :type Linear%20Color%20Structure) (DrawTime :type Float%20%28single-precision%29) (WorldContextObj :type Scene%20Component%20Object%20Reference))
  (bind (_outhit _returnvalue) (Collision|LineTraceByChannel WorldContextObj (Transformation|GetWorldLocation FromActor) (Transformation|GetWorldLocation ToActor) TraceChannel bTraceComplex ActorsToIgnore DrawDebugType IgnoreSelf TraceColor TraceHitColor DrawTime))
  (return _outhit _returnvalue))

(fn TracebyChfromActor
  (params (FromActor :type Scene%20Component%20Object%20Reference) (End :type Vector) (TraceChannel :type ETraceTypeQuery%20Enum :default "TraceTypeQuery1") (bTraceComplex :type Boolean) (ActorsToIgnore :type Array%20of%20Actor%20Object%20References) (DrawDebugType :type EDrawDebugTrace%20Enum :default "None") (IgnoreSelf :type Boolean) (TraceColor :type Linear%20Color%20Structure) (TraceHitColor :type Linear%20Color%20Structure) (DrawTime :type Float%20%28single-precision%29) (WorldContextObj :type Scene%20Component%20Object%20Reference))
  (bind (_outhit _returnvalue) (Collision|LineTraceByChannel WorldContextObj (Transformation|GetWorldLocation FromActor) End TraceChannel bTraceComplex ActorsToIgnore DrawDebugType IgnoreSelf TraceColor TraceHitColor DrawTime))
  (return _outhit _returnvalue))

(fn GWL
  (params (Target :type Scene%20Component%20Object%20Reference))
  (return (Transformation|GetWorldLocation Target)))

(fn IsValidGatewithReturnFunc
  (params (Object :type Object%20Object%20Reference))
  (if (Utilities|IsValid Object)
    (return Object)))

(fn AppendwithSpaces
  (params (1 :type String) (2 :type String) (3 :type String) (4 :type String))
  (return (Utilities|String|Append 1 " " 2 " " 3 " " 4)))