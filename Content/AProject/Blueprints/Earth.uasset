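; Earth actor whose atmosphere glow responds to values from a frequency analyzer.
; The construction script creates a dynamic material instance from the cosmos Earth material on the static mesh.
; On BeginPlay it binds to the analyzer's frequency dispatcher, and each received value is remapped with clamping to drive the material's AtmospherePower parameter.
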(event Custom|ReceivedFreqs
  (params (FreqValue :type Float%20%28single-precision%29) (WorldTimeDilation :type Float%20%28single-precision%29))
  ;[0 0.2734 1 0.3] AtmoSphereDynamicPower
  (Rendering|Material|SetScalarParameterValue (Variables|Default|GetDynaMat) "AtmospherePower" (Math|Float|MapRangeClamped FreqValue 0.0 1e+01 3.0 (Variables|Default|GetMax)) :!class /Script/Engine.MaterialInstanceDynamic))

(event EventBeginPlay
  ;[0 0.2734 1 0.3] AtmoSphereDynamicPower
  (bind _freq_analyzerref (Utilities|GetFreqAnalyzer))
  (EventDispatchers|AssignCallFreqDispatch _freq_analyzerref (delegate Custom|ReceivedFreqs)))

(fn ConstructionScript
  (bind _returnvalue (Rendering|Material|CreateDynamicMaterialInstance (Variables|Default|GetStaticMesh) 0 "/Game/AProject/Assets/Materials/EarthCoolMat_Inst_Cosmos.EarthCoolMat_Inst_Cosmos" "None" :!class /Script/Engine.PrimitiveComponent))
  (Variables|Default|SetDynaMat _returnvalue))