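; PermutionsGenerator is a Blueprint test that, despite its name, builds and prints a growing string rather than producing permutations.
; On BeginPlay it runs a ten-thousand-step loop over InputArray, appending each element as text to TempFinalStringArray and printing it twice per step.
; The string is never reset, and NewFunction0, with an unused Split node, is an empty stub.
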(event EventBeginPlay
  (for _index (range 0 10000)
    (for _array_element (Variables|Default|GetInputArray)
      (bind _output_get (Variables|Default|SetTempFinalStringArray (Utilities|String|Append (Variables|Default|GetTempFinalStringArray) (Utilities|String|ToString(Integer) _array_element))))
      (Development|PrintString _output_get)
      (Development|PrintString _output_get))))

(fn ConstructionScript)

(fn NewFunction0
  (params (SourceString :type String)))