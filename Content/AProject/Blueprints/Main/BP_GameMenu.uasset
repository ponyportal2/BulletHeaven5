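; Game menu actor with two shootable options that start the game by streaming in either the Horizontal or Vertical level.
; GotShot converts the hit component's name to an option index, broadcasts game start, disables option collision and hides both options.
; The Horizontal path also sends the player capsule a rotation and spawns blood bursts at both options.
; BeginPlay currently auto-selects Horizontal after a two-frame delay, bypassing the choice.
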(event EventBeginPlay
  (bind _bloodscale (Variables|Default|GetBloodScale))
  (bind _bloodmultiplier (Variables|Default|GetBloodMultiplier))
  (bind _returnvalue (* _bloodscale _bloodmultiplier))
  (Utilities|2FramesDelay
    (:Completed
      (Default|CallGameStarted)
      (Utilities|DisableCollisionandVisibility (Utilities|Array|MakeArray (Variables|Default|Get0) (Variables|Default|Get1)) (Utilities|Array|MakeArray (Variables|Default|GetOption0) (Variables|Default|GetOption1)))
      (Game|LoadStreamLevel(byName) (Variables|Default|GetHorizontal) true)
      (bind _playercapsule (Utilities|GetPlayerCapsule))
      (Class|BPIIInitialRotation|InitialRotation(Message) _playercapsule -90)
      (Utilities|FlowControl|Sequence
        (:then_0
          (Effects|SpawnEmitteratLocation "/Game/AProject/Files/Effects/ParticleSystems/P_BodyHit.P_BodyHit" (Transformation|GetWorldLocation (Variables|Default|GetOption0)) "0, 0, 0" _returnvalue true "AutoRelease"))
        (:then_1
          (Effects|SpawnEmitteratLocation "/Game/AProject/Files/Effects/ParticleSystems/P_BodyHit.P_BodyHit" (Transformation|GetWorldLocation (Variables|Default|GetOption1)) "0, 0, 0" _returnvalue true "AutoRelease"))))))

(event EventGotShot
  (params (HitCOmponent :type Actor%20Component%20Object%20Reference))
  (bind _returnvalue (Utilities|GetObjectName HitCOmponent))
  (bind _bloodscale (Variables|Default|GetBloodScale))
  (bind _0 (Variables|Default|Get0))
  (bind _1 (Variables|Default|Get1))
  (bind _option0 (Variables|Default|GetOption0))
  (bind _option1 (Variables|Default|GetOption1))
  (bind _bloodmultiplier (Variables|Default|GetBloodMultiplier))
  (bind _returnvalue_2 (Math|Conversions|ToInteger(Byte) _returnvalue))
  (bind _returnvalue_3 (* _bloodscale _bloodmultiplier))
  (bind _array (Utilities|Array|MakeArray _0 _1))
  (bind _array_2 (Utilities|Array|MakeArray _option0 _option1))
  (Default|CallGameStarted _returnvalue_2)
  (switch int _returnvalue_2
    (:0
      (Utilities|DisableCollisionandVisibility _array _array_2)
      (Game|LoadStreamLevel(byName) (Variables|Default|GetHorizontal) true)
      (bind _playercapsule (Utilities|GetPlayerCapsule))
      (Class|BPIIInitialRotation|InitialRotation(Message) _playercapsule -90)
      (Utilities|FlowControl|Sequence
        (:then_0
          (Effects|SpawnEmitteratLocation "/Game/AProject/Files/Effects/ParticleSystems/P_BodyHit.P_BodyHit" (Transformation|GetWorldLocation (Variables|Default|GetOption0)) "0, 0, 0" _returnvalue_3 true "AutoRelease"))
        (:then_1
          (Effects|SpawnEmitteratLocation "/Game/AProject/Files/Effects/ParticleSystems/P_BodyHit.P_BodyHit" (Transformation|GetWorldLocation (Variables|Default|GetOption1)) "0, 0, 0" _returnvalue_3 true "AutoRelease"))))
    (:1
      (Utilities|DisableCollisionandVisibility _array _array_2)
      (Game|LoadStreamLevel(byName) (Variables|Default|GetVertical) true))))

(fn ConstructionScript)