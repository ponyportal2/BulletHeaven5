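; BP_PlayerPistol is the player's pistol, firing BP_ProjectileBasePlayer projectiles from the skeletal mesh's Muzzle socket along a supplied direction.
; ShootingTheWeapon spawns a scaled-down projectile, hands it the player reference and always returns false.
; The Shood event duplicates that spawn without setting the player reference.
; A separate DebugSpawn macro waits briefly, then calls GotIt on the first BP_Planet in the level.
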(event Custom|Shood
  (params (Vector :type Vector))
  (Game|SpawnActorfromClass "/Game/AProject/Blueprints/BP_ProjectileBasePlayer.BP_ProjectileBasePlayer_C" (Math|Transform|MakeTransform (.location (Transformation|GetSocketTransform (Variables|Default|GetSkeletalMesh) "Muzzle" "RTS_World")) (Math|Conversions|RotationFromXVector Vector) (Math|Conversions|ToVector(Float) (CallFunction|LocalFloat 0.7))) "AlwaysSpawn" 0 0))

(fn ConstructionScript)

(fn ShootingtheWeapon
  (params (ForwardVector :type Vector :default "0, 0, 0") (PlayerRef :type BP%20Gear%20VR%20Pawn%20Object%20Reference))
  (bind _returnvalue (Game|SpawnActorfromClass "/Game/AProject/Blueprints/BP_ProjectileBasePlayer.BP_ProjectileBasePlayer_C" (Math|Transform|MakeTransform (.location (Transformation|GetSocketTransform (Variables|Default|GetSkeletalMesh) "Muzzle" "RTS_World")) (Math|Conversions|RotationFromXVector ForwardVector) (Math|Conversions|ToVector(Float) (CallFunction|LocalFloat 0.7))) "AlwaysSpawn" 0 0))
  (Variables|/Game/AProject/Blueprints/BP_ProjectileBase.BP_ProjectileBase_C|SetPlayerRef _returnvalue PlayerRef)
  (return false))