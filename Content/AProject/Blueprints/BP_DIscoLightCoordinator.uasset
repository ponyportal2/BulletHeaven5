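; Coordinator Blueprint that makes the point lights of all BP_ALight actors react to audio frequency data as disco lighting.
; LightAdded gathers the light components and switches them to unitless intensity.
; BeginPlay finds BP_FreqAnalyzer, retrying if the cast fails, and binds to its frequency dispatcher.
; Each received value randomizes color with capped green, scales intensity by two modifiers, and maps attenuation radius within a clamped range.
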(event Custom|FreqReceived
  (params (FreqValue :type Float%20%28single-precision%29) (WorldTimeDilation :type Float%20%28single-precision%29))
  ;[0.7813 0 1 0.3] FreqReceived
  (Variables|Default|SetFreqValue FreqValue)
  ;;[1 0.6797 0 0.3] Color
  (CallFunction|ColorFunc)
  ;;[0 1 0.1797 0.3] Intensity
  (CallFunction|IntensFunc)
  ;;;[0 0.7187 1 0.3] Attenuation
  (CallFunction|AttenFunc))

(event EventBeginPlay
  ;[1 0.1641 0 0.3] BeginPlay
  ;[0 1 0.1328 0.3] Getter
  (bind _freq_analyzerref (Utilities|GetFreqAnalyzer))
  ;[0.6875 0 1 0.3] AssignOnFreqDispatch
  (EventDispatchers|BindEventtoCallFreqDispatch _freq_analyzerref (EventDispatchers|CreateEvent :!event Custom|FreqReceived)))

(event EventLightAdded
  ;[0.7109 1 0 0.3] LightGetters
  (bind _outactors (Actor|GetAllActorsOfClass "/Game/AProject/Blueprints/BP_ALight.BP_ALight_C"))
  (bind _output_get (Variables|Default|SetPointLights _outactors))
  (for _array_element _output_get
    (Class|LocalLightComponent|SetIntensityUnits (Variables|/Game/AProject/Blueprints/BP_ALight.BP_ALight_C|GetLait _array_element) "Unitless")
    (Utilities|Array|AddUnique (Variables|Default|GetPointLightComps) (Variables|/Game/AProject/Blueprints/BP_ALight.BP_ALight_C|GetLait _array_element))))

(fn ConstructionScript)

(fn GetFreqAnalyzer
  (bind _outactors (Actor|GetAllActorsOfClass "/Game/AProject/Blueprints/BP_FreqAnalyzer.BP_FreqAnalyzer_C" :!label _label))
  (bind _asbp_freq_analyzer (Utilities|Casting|CastToBP_FreqAnalyzer (Utilities|Array|Get(acopy) _outactors))
    (:then
      (bind _output_get (Variables|Default|SetFreqAnalyzerRef _asbp_freq_analyzer))
      (return _output_get))
    (:CastFailed
      (goto _label))))

(fn ColorFunc
  ;[1 1 1] Color
  (Rendering|Components|Light|SetLightColor (Variables|Default|GetPointLightComps) (Utilities|Struct|MakeLinearColor (Math|Random|RandomFloat) (Math|Random|RandomFloatinRange 0.0 0.5) (Math|Random|RandomFloat) 1.0) true))

(fn IntensFunc
  (Rendering|Components|Light|SetIntensity (Variables|Default|GetPointLightComps) (|((x*y)*z) (Variables|Default|GetFreqValue) (Variables|Default|GetInitial%20Intensity%20Modifier) (Variables|Default|GetIntensityModifier))))

(fn AttenFunc
  (Rendering|Lighting|SetAttenuationRadius (Variables|Default|GetPointLightComps) (Math|Float|MapRangeClamped (Variables|Default|GetFreqValue) 0.0 1.0 (Variables|Default|GetMinAttenuation) (Variables|Default|GetMaxAttenuation))))