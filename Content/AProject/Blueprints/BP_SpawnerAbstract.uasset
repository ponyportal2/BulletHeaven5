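; BP_SpawnerAbstract is a base spawner that triggers spawning repeatedly at random intervals, leaving Spawn empty for children to implement.
; BeginPlay spawns immediately, and each spawn event re-arms a one-shot timer with a random delay between min and max.
; RandomInBoxNoOverride returns a random point inside the Box component.
; The game-menu game-started binding is disconnected and its event is empty, so spawning starts at BeginPlay.
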(event Custom|CreateAThingEvent
  ;[0.8281 1 0 0.5] CreateGuard/Obstacle etc.
  (CallFunction|Spawn)
  (Variables|ParentVars|SetTimerDelayValue (Math|Random|RandomFloatinRange (Variables|Default|GetMinSpawnDelay) (Variables|Default|GetMaxSpawnDelay)))
  (CallFunction|Timer (EventDispatchers|CreateEvent :!event Custom|CreateAThingEvent) false (stale EventBeginPlay _output_get)))

(event Custom|GameStartedEvent
  (params (TrackNumber :type Integer))
  ;[0 0 0] Setup with GetterDOP
  ;;[0.2656 0 1 0.5] Getter
)

(event EventBeginPlay
  ;[1 0.1875 0 0.5] BeginPlay
  (CallFunction|CreateAThingEvent)
  (bind _output_get (Variables|ParentVars|SetTimerDelayValue (Math|Random|RandomFloatinRange (Variables|Default|GetMinSpawnDelay) (Variables|Default|GetMaxSpawnDelay))))
  (CallFunction|Timer (EventDispatchers|CreateEvent :!event Custom|CreateAThingEvent) false _output_get))

(fn ConstructionScript)

(fn RandominBoxNoOverride
  (return (Math|Random|RandomPointinBoundingBox (Transformation|GetWorldLocation (Variables|Default|GetBox)) (Components|Box|GetScaledBoxExtent (Variables|Default|GetBox)))))

(fn Spawn)